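; Game mode Blueprint that runs a minutes-and-seconds countdown for a game in the AR content and triggers a loss when time runs out.
; Tick feeds a one-second Delay that paces each decrement of Sec, with Min dropping and Sec resetting whenever Sec reaches zero.
; When both reach zero, it casts the player pawn to BP_Pawn and calls Perdiste.
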(event EventBeginPlay)

(event EventTick
  (params (DeltaSeconds :type Float%20%28single-precision%29))
  ;[1 1 1] timer
  (Utilities|FlowControl|Delay 1.0)
  (bind _result (Math|Integer|DecrementInt (Variables|Default|GetSec))
    (:%20%20
      (Variables|Default|SetSec _result)
      (if (not (!= (Variables|Default|GetSec) 0))
        (if (> (Variables|Default|GetMin) 0)
          (bind _result_2 (Math|Integer|DecrementInt (Variables|Default|GetMin))
            (:%20%20
              (Variables|Default|SetMin _result_2)
              (Variables|Default|SetSec 59)))
          (else
            (bind _asbp_pawn (Utilities|Casting|CastToBP_Pawn (Game|Player|GetPlayerPawn 0)))
            (Default|Perdiste _asbp_pawn)))))))

(fn ConstructionScript)